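; BP_TestButton is an interactable button that checks whether the player has matched all paintings and prints a win or lose message.
; Looking at it shows its name on the ExplorerHUD and swaps its material; Tick restores the material once the HUD message hides.
; Use animates the press, then treats PaintingDataTable row names as actor tags to find each BP_Painting and test IsMatched.
; Some disconnected debug-print logic remains unused.
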(event EventLookat
  (bind _explorerhud (Variables|Default|GetExplorerHUD))
  ;[1 1 1] Light up the button if we're looking at it
  (Variables|/Game/MuseumExplorer/Blueprints/ExplorerHUD.ExplorerHUD_C|Setcurrent_msg _explorerhud (Variables|Default|Getitem_name))
  (Variables|/Game/MuseumExplorer/Blueprints/ExplorerHUD.ExplorerHUD_C|Setshow_msg _explorerhud true)
  (Rendering|Material|SetMaterial (Variables|Default|GetButton) 0 "/Game/FirstPerson/Meshes/BaseMaterial.BaseMaterial"))

(event EventUse
  (bind _button (Variables|Default|GetButton))
  ;[1 1 1] Press the button
  (Components|MoveComponentTo _button "0, 0,118.000000" "0, 0,0.000000" true true 0.2 false)
  (Components|MoveComponentTo _button "0, 0,123.000000" "0, 0,0.000000" true true 0.2 false)
  (Variables|Default|Setall_matched true)
  (bind _outrownames (DataTable|GetDataTableRowNames "/Game/MuseumExplorer/Data/PaintingDataTable.PaintingDataTable"))
  (for _array_element _outrownames
    (bind _outactors (Actor|GetAllActorswithTag _array_element))
    (for _array_element_2 _outactors
      (bind _asbp_painting (Utilities|Casting|CastToBP_Painting _array_element_2))
      (if (not (Variables|/Game/MuseumExplorer/Blueprints/BP_Painting.BP_Painting_C|Getis_matched _asbp_painting))
        (Variables|Default|Setall_matched false))))
  (if (Variables|Default|Getall_matched)
    (Development|PrintString "YOU WON!!!")
    (else
      (Development|PrintString "YOU LOSE :( :( :("))))

(event EventTick
  (params (DeltaSeconds :type Float%20%28single-precision%29))
  ;[1 1 1] Unlight the button if we're looking away
  (if (not (Variables|/Game/MuseumExplorer/Blueprints/ExplorerHUD.ExplorerHUD_C|Getshow_msg (Variables|Default|GetExplorerHUD)))
    (Rendering|Material|SetMaterial (Variables|Default|GetButton) 0 "/Game/StarterContent/Materials/M_Basic_Floor.M_Basic_Floor")))

(event EventBeginPlay
  ;[1 1 1] Grab a reference to the ExplorerHUD
  (bind _asexplorer_hud (Utilities|Casting|CastToExplorerHUD (HUD|GetHUD (Game|GetPlayerController 0))))
  (Variables|Default|SetExplorerHUD _asexplorer_hud))

(fn ConstructionScript)

(fn GetMaxLookatDistance
  (return (Variables|Default|Getmax_look_distance)))