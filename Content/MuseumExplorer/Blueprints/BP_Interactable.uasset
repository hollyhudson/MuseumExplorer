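; BP_Interactable is an interactable item in MuseumExplorer that shows its name when looked at and disappears when used.
; Lookat casts the player's HUD to ExplorerHUD, then sets its current message to ItemName and turns the message on.
; Use prints a debug string and destroys the actor.
; GetMaxLookAtDistance exposes the item's MaxLookDistance to callers.
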(event EventUse
  (Development|PrintString "IN USE IN INTERACTABLE")
  (Actor|DestroyActor))

(event EventLookat
  (bind _asexplorer_hud (Utilities|Casting|CastToExplorerHUD (HUD|GetHUD (Game|GetPlayerController 0)))
    (:then
      (Variables|/Game/MuseumExplorer/Blueprints/ExplorerHUD.ExplorerHUD_C|Setcurrent_msg _asexplorer_hud (Variables|Default|Getitem_name))
      (Variables|/Game/MuseumExplorer/Blueprints/ExplorerHUD.ExplorerHUD_C|Setshow_msg _asexplorer_hud true))
    (:CastFailed
      (Development|PrintString "CAST TO EXPLORERHUD FAILED"))))

(fn ConstructionScript)

(fn GetMaxLookatDistance
  (return (Variables|Default|Getmax_look_distance)))