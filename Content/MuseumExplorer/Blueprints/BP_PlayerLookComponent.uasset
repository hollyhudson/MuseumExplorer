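; BP_PlayerLookComponent is a player component that tracks what the owner's camera is looking at.
; On BeginPlay it caches the owner's CameraComponent as Eye.
; Each tick it sphere-traces on the Visibility channel from Eye along its forward vector out to LookAtDistance.
; A miss clears LookatTarget; the graph has no logic for assigning a target on a hit.
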(event EventBeginPlay
  (bind _returnvalue (Components|GetOwner))
  (bind _returnvalue_2 (Actor|GetComponentbyClass _returnvalue "/Script/Engine.CameraComponent"))
  ;[1 1 1] Initialize Eye on Camera
  (Utilities|IsValid _returnvalue_2
    (:Is%20Valid
      (Variables|Default|Seteye _returnvalue_2))))

(event EventTick
  (params (DeltaSeconds :type Float%20%28single-precision%29))
  (bind _eye (Variables|Default|Geteye))
  (bind _returnvalue (Transformation|GetWorldLocation _eye))
  (bind _returnvalue_2 (Collision|SphereTraceByChannel _returnvalue (+ _returnvalue (* (Math|Vector|GetForwardVector _eye) (Variables|Default|Getlook_at_distance))) 1e+01 "TraceTypeQuery1" false 0 "None"))
  (if (not _returnvalue_2)
    (Variables|Default|Setlookat_target 0)))