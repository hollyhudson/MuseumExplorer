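; Artifact the player picks up, carries and places on painting receptacles as part of a matching mechanic.
; Use attaches it to the player's hands, or, when hands are full, checks overlapping components to snap it onto a free ArtifactReceptacle or drop it with physics.
; Placement compares MatchId with the owning BP_Painting to set IsMatched; pickup from a receptacle clears that state.
; Data table update logic is unconnected and never runs.
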(event OnComponentBeginOverlap(Sphere)
  (params (OverlappedComponent :type Primitive%20Component%20Object%20Reference) (OtherActor :type Actor%20Object%20Reference) (OtherComp :type Primitive%20Component%20Object%20Reference) (OtherBodyIndex :type Integer) (bFromSweep :type Boolean) (SweepResult :type Hit%20Result%20Structure%20%28by%20ref%29))
  (Variables|Default|Setoverlapping true))

(event OnComponentEndOverlap(Sphere)
  (params (OverlappedComponent :type Primitive%20Component%20Object%20Reference) (OtherActor :type Actor%20Object%20Reference) (OtherComp :type Primitive%20Component%20Object%20Reference) (OtherBodyIndex :type Integer))
  (Variables|Default|Setoverlapping false))

(event EventUse
  (bind _player (Variables|Default|Getplayer))
  (if (Variables|/Game/MuseumExplorer/Blueprints/ExplorerCharacter.ExplorerCharacter_C|Gethands_full (Variables|Default|Getplayer)) ; Are we carrying something already?
    (if (Variables|Default|Getoverlapping) ; Is it what we're carrying overlapping something?
      (for _array_element (Class|Actor|GetOverlappingComponents) ; What all is it overlapping?
        (if (Utilities|Enum|Equal(Enum) (Utilities|GetObjectName _array_element) "ArtifactReceptacle") ; Perhaps a pedestal?
          (bind _asbp_painting (Utilities|Casting|CastToBP_Painting (Components|GetOwner _array_element)))
          (if (Variables|/Game/MuseumExplorer/Blueprints/BP_Painting.BP_Painting_C|Getreceptacle_full _asbp_painting) ; Is the pedestal occupied?
            ;[1 1 1] Drop artifact
            (Transformation|DetachFromActor "KeepWorld" "KeepRelative" "KeepRelative" :!label _label)
            (Physics|SetSimulatePhysics (Variables|Default|GetSphere) true)
            (Variables|/Game/MuseumExplorer/Blueprints/ExplorerCharacter.ExplorerCharacter_C|Setartifact_holding _player "None")
            (Variables|/Game/MuseumExplorer/Blueprints/ExplorerCharacter.ExplorerCharacter_C|Sethands_full _player false)
            (else
              ;[1 1 1] Place artifact on pedestal
              (Transformation|AttachComponentToComponent (Variables|Default|GetSphere) _array_element "None" "SnapToTarget" "KeepRelative" "KeepRelative" true)
              (Variables|/Game/MuseumExplorer/Blueprints/BP_Painting.BP_Painting_C|Setreceptacle_full _asbp_painting true)
              (Variables|Default|Seton_a_pedestal true)
              (Variables|/Game/MuseumExplorer/Blueprints/ExplorerCharacter.ExplorerCharacter_C|Sethands_full (Variables|Default|Getplayer) false)
              ;[1 1 1] Is it a match?
              (if (Utilities|Enum|Equal(Enum) (Variables|/Game/MuseumExplorer/Blueprints/BP_Painting.BP_Painting_C|Getmatch_id _asbp_painting) (Variables|Default|Getmatch_id))
                (Development|PrintString "IT\"S A MATCH!")
                (Variables|/Game/MuseumExplorer/Blueprints/BP_Painting.BP_Painting_C|Setis_matched _asbp_painting true)
                (else
                  (Development|PrintString "ITS NOT A MATCH :( :( :(")
                  (Variables|/Game/MuseumExplorer/Blueprints/BP_Painting.BP_Painting_C|Setis_matched _asbp_painting false)))))
          (else
            (goto _label))))
      (else
        (Transformation|DetachFromActor "KeepWorld" "KeepRelative" "KeepRelative")
        (Physics|SetSimulatePhysics (Variables|Default|GetSphere) true)
        (Variables|/Game/MuseumExplorer/Blueprints/ExplorerCharacter.ExplorerCharacter_C|Setartifact_holding _player "None")
        (Variables|/Game/MuseumExplorer/Blueprints/ExplorerCharacter.ExplorerCharacter_C|Sethands_full _player false)))
    (else
      ;[1 1 1] Pick up artifact
      (Variables|/Game/MuseumExplorer/Blueprints/ExplorerCharacter.ExplorerCharacter_C|Setartifact_holding (Variables|Default|Getplayer) (Variables|Default|Getartifact_name))
      (if (Variables|Default|Geton_a_pedestal) ; Is what we're picking up on a pedestal?
        ;;[1 1 1] Detach from pedestal first and unmatch any matches for that painting
        (bind _asbp_painting_2 (Utilities|Casting|CastToBP_Painting (Components|GetOwner (Transformation|GetAttachParent (Variables|Default|GetSphere)))))
        (Variables|/Game/MuseumExplorer/Blueprints/BP_Painting.BP_Painting_C|Setreceptacle_full _asbp_painting_2 false)
        (Variables|Default|Seton_a_pedestal false)
        (Variables|/Game/MuseumExplorer/Blueprints/BP_Painting.BP_Painting_C|Setis_matched _asbp_painting_2 false))
      (Physics|SetSimulatePhysics (Variables|Default|GetSphere) false)
      (Transformation|AttachComponentToComponent (Variables|/Game/MuseumExplorer/Blueprints/ExplorerCharacter.ExplorerCharacter_C|GetAttachmentPoint (Variables|Default|Getplayer)) "None" "SnapToTarget" "KeepRelative" "KeepRelative" true)
      (Variables|/Game/MuseumExplorer/Blueprints/ExplorerCharacter.ExplorerCharacter_C|Sethands_full (Variables|Default|Getplayer) true)
      (Variables|Default|Seton_a_pedestal false))))

(event EventBeginPlay
  ;[1 1 1] Get a reference to the player for the artifact to use
  (bind _asexplorer_character (Utilities|Casting|CastToExplorerCharacter (Game|Player|GetPlayerPawn 0)))
  (Variables|Default|Setplayer _asexplorer_character))

(fn ConstructionScript
  (|CallParentFunction))

(fn GetMaxLookatDistance
  (return (Variables|Default|Getmax_look_distance)))